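; BP_Projectile is a tumbling projectile that launches itself at the BP_Boat actor.
; On BeginPlay it computes an intercept velocity with SuggestProjectileVelocityMovingTarget, using a fixed offset and flight time, and feeds it to ProjectileMovement.
; It also rolls a random rotator that Tick adds to the mesh every frame, independent of delta time.
; Taking damage spawns DeathEffect and destroys it, while hits only print the other actor's name.
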(event `self.ReceiveBeginPlay`
  (bind _returnvalue (`GameplayStatics.GetActorOfClass` "/Game/BP_Boat.BP_Boat_C"))
  (bind _outlaunchvelocity (`GameplayStatics.SuggestProjectileVelocity_MovingTarget` (`self.K2_GetActorLocation`) _returnvalue (250.0 0.0 50.0) 0.0 1.5 "None"))
  (set `MovementComponent.Velocity` _outlaunchvelocity (`self.ProjectileMovement`))
  (bind _return (`self.GetRandomRotator`))
  (set `self.Rotator` _return))

(event `self.ReceiveHit`
  (params (MyComp :type "PrimitiveComponent Object Reference") (Other :type "Actor Object Reference") (OtherComp :type "PrimitiveComponent Object Reference") (bSelfMoved :type Boolean) (HitLocation :type "Vector Structure") (HitNormal :type "Vector Structure") (NormalImpulse :type "Vector Structure") (Hit :type "HitResult Structure (by ref)"))
  (`KismetSystemLibrary.PrintString` (`KismetSystemLibrary.GetDisplayName` Other)))

(event `Damage`
  (`|SpawnActorFromClass` (`self.DeathEffect`) (`self.GetTransform`) "Undefined" "MultiplyWithRoot" null null)
  (`self.K2_DestroyActor`))

(event `self.ReceiveTick`
  (params (DeltaSeconds :type "Float (single-precision)"))
  (`SceneComponent.K2_AddRelativeRotation` (`self.StaticMesh`) (`self.Rotator`) false false))

(fn `GetRandomFloat`
  (returns (Return :type "Float (double-precision)"))
  (return (`KismetMathLibrary.RandomFloatInRange` (`self.MinFloat`) (`self.MaxFloat`))))

(fn `GetRandomRotator`
  (returns (Return :type "Rotator Structure"))
  (bind _return (`self.GetRandomFloat`))
  (bind _return_2 (`self.GetRandomFloat`))
  (bind _return_3 (`self.GetRandomFloat`))
  (return (`KismetMathLibrary.MakeRotator` _return _return_2 _return_3)))

(fn `UserConstructionScript`)