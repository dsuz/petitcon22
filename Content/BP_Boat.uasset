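; BP_Boat is an actor that rocks its Boat component to give it a bobbing motion.
; A looping timeline, started from Tick, drives world pitch from its Angle curve scaled by the current amplitude, preserving roll and yaw.
; Each time the timeline finishes, it picks a new random amplitude between the configured minimum and maximum and replays, so successive rocking cycles vary in strength.
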(event `self.ReceiveTick`
  (params (DeltaSeconds :type "Float (single-precision)"))
  (bind _boat (`self.Boat`))
  (bind (_returnvalue_roll _returnvalue_pitch _returnvalue_yaw) (`KismetMathLibrary.BreakRotator` (`SceneComponent.K2_GetComponentRotation` _boat)))
  (bind (_direction _angle) (`Timeline|Timeline` :!label _label)
    (:`Update`
      (`SceneComponent.K2_SetWorldRotation` _boat (`KismetMathLibrary.MakeRotator` _returnvalue_roll (* _angle (`self.CurrentAmplitude`)) _returnvalue_yaw) false false))
    (:`Finished`
      (bind _return (`self.GetRandomAmplitude`))
      (set `self.CurrentAmplitude` _return)
      (goto _label :!via `PlayFromStart`))))

(fn `GetRandomAmplitude`
  (returns (Return :type "Float (double-precision)"))
  (return (`KismetMathLibrary.RandomFloatInRange` (`self.MinAmplitude`) (`self.MaxAmplitude`))))

(fn `UserConstructionScript`)