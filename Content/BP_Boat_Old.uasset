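; Boat actor, named as an old version, that makes its BoatAnchor component follow a referenced Anchor actor.
; Each Tick it teleports BoatAnchor to the Anchor's world location and rotation.
; Unconnected leftover nodes hold abandoned physics approaches: velocity pull toward the Anchor, and torque or angular-velocity turning, with one branch picking direction from the Anchor's boat-local X.
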(event `self.ReceiveBeginPlay`)

(event `self.ReceiveTick`
  (params (DeltaSeconds :type "Float (single-precision)"))
  (bind _anchor (`self.Anchor`))
  (`SceneComponent.K2_SetWorldLocationAndRotation` (`self.BoatAnchor`) (`self.K2_GetActorLocation` _anchor) (`self.K2_GetActorRotation` _anchor) false true))

(fn `UserConstructionScript`)